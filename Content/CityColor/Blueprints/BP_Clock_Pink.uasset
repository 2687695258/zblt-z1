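; Pink clock actor that shows either the system time or a ticking custom time on an animated skeletal mesh.
; A looping Delay converts hours, minutes and seconds into hand angles and writes them to ABP_Clock_Pink every 0.05 seconds.
; When custom ticking is enabled, a parallel one-second loop advances cached time counters with 12-hour rollover.
; BeginPlay also starts the clock's animation montage.
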(event EventBeginPlay
  (bind _returnvalue (Math|DateTime|Now))
  (Utilities|FlowControl|Sequence
    (:then_0
      ;[1 1 1] 获得动画蓝图
      (bind _asabp_clock_pink (Utilities|Casting|CastToABP_Clock_Pink (Components|SkeletalMesh|GetAnimInstance (Variables|Default|GetSM_Clock_Pink))))
      (Variables|Default|SetClockPink _asabp_clock_pink))
    (:then_1
      ;[1 1 1] 自定义初始时间；使用当前时间
      (Variables|Default|SetCmTimeH (select (== (Variables|Default|GetCmTimeH) 12) 0 (Variables|Default|GetCmTimeH)))
      (Variables|Default|SetCmTimeM (select (== (Variables|Default|GetCmTimeM) 60) 0 (Variables|Default|GetCmTimeM)))
      (Variables|Default|SetCmTimeS (select (== (Variables|Default|GetCmTimeS) 60) 0 (Variables|Default|GetCmTimeS)))
      (if (Variables|Default|GetDisplayRealTime)
        (Variables|/Game/CityColor/Blueprints/ABP_Clock_Pink.ABP_Clock_Pink_C|SetHourAngle (Variables|Default|GetClockPink) (- 0.0 (+ (Math|Conversions|ToFloat(Integer) (* (select (== (select (Variables|Default|GetDisplayRealTime) (Class|KismetMathLibrary|GetHour12 _returnvalue) (Variables|Default|GetCmCacheTimeH)) 12) 0 (select (Variables|Default|GetDisplayRealTime) (Class|KismetMathLibrary|GetHour12 _returnvalue) (Variables|Default|GetCmCacheTimeH))) 30)) (* (select (Variables|Default|GetDisplayRealTime) (Class|KismetMathLibrary|GetMinute _returnvalue) (Variables|Default|GetCmCacheTimeM)) 0.5))) :!label _label)
        (Variables|/Game/CityColor/Blueprints/ABP_Clock_Pink.ABP_Clock_Pink_C|SetMinuteAngle (Variables|Default|GetClockPink) (Math|Float|MapRangeClamped (Math|Conversions|ToFloat(Integer) (select (Variables|Default|GetDisplayRealTime) (Class|KismetMathLibrary|GetMinute _returnvalue) (Variables|Default|GetCmCacheTimeM))) 0.0 6e+01 0.0 -3.6e+02))
        (Variables|/Game/CityColor/Blueprints/ABP_Clock_Pink.ABP_Clock_Pink_C|SetSecondAngle (Variables|Default|GetClockPink) (Math|Float|MapRangeClamped (Math|Conversions|ToFloat(Integer) (select (Variables|Default|GetDisplayRealTime) (Class|KismetMathLibrary|GetSecond _returnvalue) (Variables|Default|GetCmCacheTimeS))) 0.0 6e+01 0.0 -3.6e+02))
        (Utilities|FlowControl|Delay 0.05)
        (goto _label)
        (elif (Variables|Default|GetTickCustomTime)
          (Utilities|FlowControl|Sequence
            (:then_0
              (Utilities|FlowControl|Delay 1.0 :!label _label_2)
              (if (< (Variables|Default|GetCmCacheTimeS) 59)
                (Math|Integer|IncrementInt (Variables|Default|GetCmCacheTimeS)
                  (:%20%20
                    (goto _label_2)))
                (else
                  (Variables|Default|SetCmCacheTimeS 0)
                  (if (< (Variables|Default|GetCmCacheTimeM) 59)
                    (Math|Integer|IncrementInt (Variables|Default|GetCmCacheTimeM)
                      (:%20%20
                        (goto _label_2)))
                    (else
                      (Variables|Default|SetCmCacheTimeM 0)
                      (if (< (Variables|Default|GetCmCacheTimeH) 11)
                        (Math|Integer|IncrementInt (Variables|Default|GetCmCacheTimeH)
                          (:%20%20
                            (goto _label_2)))
                        (else
                          (Variables|Default|SetCmCacheTimeH 0)
                          (goto _label_2))))))))
            (:then_1
              (goto _label))))))
    (:then_2
      (Animation|Montage|PlayMontage (Variables|Default|GetSM_Clock_Pink) "/Game/CityColor/Animation/AM_Clock_Pink_Anim_Montage.AM_Clock_Pink_Anim_Montage"))))

(fn ConstructionScript)