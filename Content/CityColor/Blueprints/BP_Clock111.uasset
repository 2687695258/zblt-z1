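; Clock actor that shows real or custom time by driving hour, minute and second angles in its skeletal mesh's ABP_Clock007 animation Blueprint.
; On BeginPlay it caches that anim instance and the custom start time, then a short Delay loop converts the time to angles.
; A parallel one-second Delay loop advances custom time on a 12-hour cycle.
; With both DisplayRealTime and TickCustomTime off, the angles are never written.
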(event EventBeginPlay
  (bind _returnvalue (Math|DateTime|Now))
  (bind _customtimehours (Variables|Default|GetCustomTimeHours))
  (bind _customtimeseconds (Variables|Default|GetCustomTimeSeconds))
  (bind _customtimeminutes (Variables|Default|GetCustomTimeMinutes))
  (Utilities|FlowControl|Sequence
    (:then_0
      ;[1 1 1] 获得动画蓝图
      (bind _asabp_clock_007 (Utilities|Casting|CastToABP_Clock007 (Components|SkeletalMesh|GetAnimInstance (Variables|Default|GetSkeletalMesh))))
      (Variables|Default|SetABP%20Clock%20007 _asabp_clock_007))
    (:then_1
      ;[1 1 1] 自定义初始时间；使用当前时间
      (Variables|Default|SetCustomTimeCacheHour (select (== _customtimehours 12) 0 _customtimehours))
      (Variables|Default|SetCustomTimeCacheMinute (select (== _customtimeminutes 60) 0 _customtimeminutes))
      (Variables|Default|SetCustomTimeCacheSecond (select (== _customtimeseconds 60) 0 _customtimeseconds))
      (if (Variables|Default|GetDisplayRealTime)
        (Variables|/Game/CityColor/Blueprints/ABP_Clock007.ABP_Clock007_C|SetHourAngle (Variables|Default|GetABP%20Clock%20007) (- 0.0 (+ (Math|Conversions|ToFloat(Integer) (* (+ (select (== (select (Variables|Default|GetDisplayRealTime) (Class|KismetMathLibrary|GetHour12 _returnvalue) (Variables|Default|GetCustomTimeCacheHour)) 12) 0 (select (Variables|Default|GetDisplayRealTime) (Class|KismetMathLibrary|GetHour12 _returnvalue) (Variables|Default|GetCustomTimeCacheHour))) 10) 30)) (* (select (Variables|Default|GetDisplayRealTime) (Class|KismetMathLibrary|GetMinute _returnvalue) (Variables|Default|GetCustomTimeCacheMinute)) 0.5))) :!label _label)
        (Variables|/Game/CityColor/Blueprints/ABP_Clock007.ABP_Clock007_C|SetMinuteAngle (Variables|Default|GetABP%20Clock%20007) (- 0.0 (+ (* (select (Variables|Default|GetDisplayRealTime) (Class|KismetMathLibrary|GetMinute _returnvalue) (Variables|Default|GetCustomTimeCacheMinute)) 6.0) 3e+02)))
        (Variables|/Game/CityColor/Blueprints/ABP_Clock007.ABP_Clock007_C|SetSecondAngle (Variables|Default|GetABP%20Clock%20007) (Math|Float|MapRangeClamped (Math|Conversions|ToFloat(Integer) (select (Variables|Default|GetDisplayRealTime) (Class|KismetMathLibrary|GetSecond _returnvalue) (Variables|Default|GetCustomTimeCacheSecond))) 0.0 6e+01 0.0 -3.6e+02))
        (Utilities|FlowControl|Delay 0.05)
        (goto _label)
        (elif (Variables|Default|GetTickCustomTime)
          (Utilities|FlowControl|Sequence
            (:then_0
              (Utilities|FlowControl|Delay 1.0 :!label _label_2)
              (if (< (Variables|Default|GetCustomTimeCacheSecond) 59)
                (Math|Integer|IncrementInt (Variables|Default|GetCustomTimeCacheSecond)
                  (:%20%20
                    (goto _label_2)))
                (else
                  (Variables|Default|SetCustomTimeCacheSecond 0)
                  (if (< (Variables|Default|GetCustomTimeCacheMinute) 59)
                    (Math|Integer|IncrementInt (Variables|Default|GetCustomTimeCacheMinute)
                      (:%20%20
                        (goto _label_2)))
                    (else
                      (Variables|Default|SetCustomTimeCacheMinute 0)
                      (if (< (Variables|Default|GetCustomTimeCacheHour) 11)
                        (Math|Integer|IncrementInt (Variables|Default|GetCustomTimeCacheHour)
                          (:%20%20
                            (goto _label_2)))
                        (else
                          (Variables|Default|SetCustomTimeCacheHour 0)
                          (goto _label_2))))))))
            (:then_1
              (goto _label))))))))

(fn ConstructionScript)